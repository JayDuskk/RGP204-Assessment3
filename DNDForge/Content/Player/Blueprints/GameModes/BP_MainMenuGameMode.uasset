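; Main menu game mode that sets up the menu screen when play begins and writes a race save slot.
; On BeginPlay it first creates a RaceSaveGame with hardcoded Teifling race info and saves it to a slot named from the race name plus a "_RaceSlot" suffix.
; It then adds the MainMenu widget to the viewport, switches input to UI only and shows the mouse cursor.
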(event `self.ReceiveBeginPlay`
  (bind _returnvalue (`GameplayStatics.GetPlayerController` 0))
  (`|ExecutionSequence`
    (:`then_0`
      (bind _returnvalue_2 (`GameplayStatics.CreateSaveGameObject` "/Game/API/Race/RaceSaveGame.RaceSaveGame_C"))
      (bind _output_get (set `/Game/API/Race/RaceSaveGame.RaceInfo` (make `/Game/Player/Blueprints/CharacterInfo/RaceInfo_Struct` "Teifling" "Demoinc Humanoid") _returnvalue_2))
      (`GameplayStatics.SaveGameToSlot` _returnvalue_2 (`KismetStringLibrary.Concat_StrStr` (`KismetTextLibrary.Conv_TextToString` (`.Name_6_BAC5623444AC469E4FF1C7B3597618B4` (break `/Game/Player/Blueprints/CharacterInfo/RaceInfo_Struct` _output_get))) "_RaceSlot")))
    (:`then_1`
      (bind _returnvalue_3 (`|CreateWidget` "/Game/Player/UI-UX/MainMenu.MainMenu_C"))
      (`UserWidget.AddToViewport` _returnvalue_3 0)
      (`WidgetBlueprintLibrary.SetInputMode_UIOnlyEx` _returnvalue null)
      (set `PlayerController.bShowMouseCursor` true _returnvalue))))

(fn `UserConstructionScript`)