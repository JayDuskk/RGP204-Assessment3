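; BP_Enemy_AI is an enemy that chases the player and hurts them on contact.
; Pawn sensing sets a seen flag that is never cleared here, letting FollowPlayer clear StandingStill and start an AI move toward the player.
; Capsule hits on the first-person character subtract fixed health directly from it, then call FollowPlayer again.
; Incoming damage reduces the enemy's Health and destroys it when none would remain.
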(event `self.PawnSensing.OnSeePawn`
  (params (Pawn :type "Pawn Object Reference"))
  (set `self.IsSeeingPlayer` true)
  (`self.FollowPlayer`))

(event `self.ReceiveAnyDamage`
  (params (Damage :type "Float (single-precision)") (DamageType :type "DamageType Object Reference") (InstigatedBy :type "Controller Object Reference") (DamageCauser :type "Actor Object Reference"))
  (bind _returnvalue (- (`self.Health`) Damage))
  (if (> _returnvalue 0.0)
    (set `self.Health` _returnvalue)
    (else
      (`self.K2_DestroyActor`))))

(event `self.ReceiveBeginPlay`
  (`|ExecutionSequence`
    (:`then_0`
      (set `self.StandingStill` true))
    (:`then_1`
      (set `self.NumberEnemyKilled` 0.0))
    (:`then_2`
      (`self.FollowPlayer`))))

(event `FollowPlayer`
  (if (`self.IsSeeingPlayer`)
    (set `self.StandingStill` false)
    (`|AIMoveTo` self (0.0 0.0 0.0) (`GameplayStatics.GetPlayerCharacter` 0))))

(event `self.CapsuleComponent.OnComponentHit`
  (params (HitComponent :type "PrimitiveComponent Object Reference") (OtherActor :type "Actor Object Reference") (OtherComp :type "PrimitiveComponent Object Reference") (NormalImpulse :type "Vector Structure") (Hit :type "HitResult Structure (by ref)"))
  (bind _asbp_first_person_character (cast `/Game/FirstPerson/Blueprints/BP_FirstPersonCharacter` OtherActor))
  (bind _output_get (set `self.Character` _asbp_first_person_character))
  (set `/Game/FirstPerson/Blueprints/BP_FirstPersonCharacter.CharacterHealth` (- (`/Game/FirstPerson/Blueprints/BP_FirstPersonCharacter.CharacterHealth` _output_get) 10.0) _output_get)
  (`self.FollowPlayer`))

(fn `UserConstructionScript`)